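; Example pickup actor for EasyMultiSave that a character collects into its inventory by overlapping its box.
; Overlaps only count once the game mode finishes loading, checked through a library function, so loading cannot trigger a pickup.
; Pickup passes the item's inventory data to the EMS_Character, then sets a disabled flag that hides the actor and turns off box collision.
; ActorLoaded reapplies that hidden and collision state after a load.
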(event OnComponentBeginOverlap(Box)
  (params (OverlappedComponent :type Primitive%20Component%20Object%20Reference) (OtherActor :type Actor%20Object%20Reference) (OtherComp :type Primitive%20Component%20Object%20Reference) (OtherBodyIndex :type Integer) (bFromSweep :type Boolean) (SweepResult :type Hit%20Result%20Structure%20%28by%20ref%29))
  (if (CallFunction|HasEMSGameModeLoadingCompleted) ; Prevent pickup before loading has completed\nwith a simple check from a Bluepront Lib Function
    (bind _asems_character (Utilities|Casting|CastToEMS_Character OtherActor))
    (CallFunction|AddtoInventory _asems_character)))

(event Custom|Add%20To%20Inventory
  (params (Character :type EMS%20Character%20Object%20Reference))
  (Default|AddActortoInventory Character (Variables|Default|GetInventoryData) true)
  (Variables|Saved|SetbIsDisabled true)
  (CallFunction|CheckActorStatus))

(event EventActorLoaded
  (CallFunction|CheckActorStatus))

(event EventBeginPlay
  (Variables|Default|SetInventoryData (Utilities|Struct|MakeEMS_OwnedActorStruct (Utilities|Struct|BreakEMS_OwnedActorStruct (Variables|Default|GetInventoryData)) (CallFunction|MakeEMSExampleStruct))))

(fn ConstructionScript)

(fn CheckActorStatus
  (bind _bisdisabled (Variables|Saved|GetbIsDisabled))
  (bind _box (Variables|Components|GetBox))
  (Rendering|SetActorHiddenInGame _bisdisabled)
  (if _bisdisabled
    (Collision|SetCollisionEnabled _box "NoCollision")
    (else
      (Collision|SetCollisionEnabled _box "QueryOnly"))))

(fn ComponentstoSave
  (return 0))