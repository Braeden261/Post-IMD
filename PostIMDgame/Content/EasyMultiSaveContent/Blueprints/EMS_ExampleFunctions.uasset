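; Blueprint function library of helpers for the Easy Multi Save example content.
; It builds a randomized EMS example struct with scalars, nested structs, arrays, a vector and a transform, plus a random opaque color.
; Getters cast the persistent save to the example save game and the game mode to EMS_GameMode.
; A final check reads that game mode's LoadComplete flag to report whether loading has finished.
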(fn MakeEMSExampleStruct
  (bind _returnvalue (Math|Random|RandomIntegerinRange 5 50000))
  (bind _returnvalue_2 (Math|Random|RandomIntegerinRange 5 50000))
  (bind _returnvalue_3 (Math|Random|RandomIntegerinRange 5 50000))
  (bind _returnvalue_4 (Math|Random|RandomIntegerinRange 5 50000))
  (bind _array (Utilities|Array|MakeArray _returnvalue_4 _returnvalue_3 _returnvalue))
  (bind _ems_intstruct (Utilities|Struct|MakeEMS_IntStruct _returnvalue_2 _array))
  (return (Utilities|Struct|MakeEMS_ExampleStruct (Math|Random|RandomBoolwithWeight 0.5) (Math|Random|RandomIntegerinRange 5 50000) (Utilities|String|MakeLiteralString "Hello World") (Math|Random|RandomFloatinRange 5.0 5e+04) (Utilities|Struct|MakeEMS_IntStruct (Math|Random|RandomIntegerinRange 5 50000) (Utilities|Array|MakeArray (Math|Random|RandomIntegerinRange 5 50000) (Math|Random|RandomIntegerinRange 5 50000) (Math|Random|RandomIntegerinRange 5 50000))) (Utilities|Array|MakeArray _ems_intstruct _ems_intstruct _ems_intstruct) (* (Math|Random|RandomUnitVector) 5e+03) (Utilities|Array|MakeArray (Math|Random|RandomIntegerinRange 5 50000) (Math|Random|RandomIntegerinRange 5 50000) (Math|Random|RandomIntegerinRange 5 50000)) (Math|Transform|MakeTransform (* (Math|Random|RandomUnitVector) 5e+03)))))

(fn GetExamplePersistentSave
  (bind _asems_example_blueprint_save_game (Utilities|Casting|CastToEMS_ExampleBlueprintSaveGame (Class|EMSFunctionLibrary|GetPersistentSave)))
  (return _asems_example_blueprint_save_game))

(fn RandomColor
  (return (Utilities|Struct|MakeLinearColor (Math|Random|RandomFloat) (Math|Random|RandomFloat) (Math|Random|RandomFloat) 1.0)))

(fn GetEMSGameMode
  (bind _asems_game_mode (Utilities|Casting|CastToEMS_GameMode (Game|GetGameMode)))
  (return _asems_game_mode))

(fn HasEMSGameModeLoadingCompleted
  (return (Variables|/Game/EasyMultiSaveContent/Blueprints/GameMode/EMS_GameMode.EMS_GameMode_C|GetbLoadComplete (CallFunction|GetEMSGameMode))))