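; Example Game Mode for the EasyMultiSave content that loads saved data whenever a player restarts, a flow geared to singleplayer.
; A macro polls every 0.1 seconds until the player controls a valid pawn, then starts an async actor load without full reload.
; It prints a test value from the globally accessible persistent save right away and flags loading as complete when the async load finishes.
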(event Custom|Load%20Persistent
  ;[1 1 1] Load Level and Player, once we have a valid pawn. This will work great for Singleplayer
  (Development|PrintString (Utilities|String|Append "Persistent Save TestInt: " (Utilities|String|ToString(Integer) (Variables|/Game/EasyMultiSaveContent/Blueprints/EMS_ExampleBlueprintSaveGame.EMS_ExampleBlueprintSaveGame_C|GetTestInt (CallFunction|GetExamplePersistentSave))))))

(event EventOnRestartPlayer
  (params (NewPlayer :type Controller%20Object%20Reference))
  ;[1 1 1] Load Level and Player, once we have a valid pawn. This will work great for Singleplayer
  (Utilities|HasValidPawn NewPlayer
    (:Is%20Valid
      (|AsyncLoadActors 3 false
        (:then
          (CallFunction|LoadPersistent))
        (:OnCompleted
          (Variables|Default|SetbLoadComplete true))))))

(fn ConstructionScript)